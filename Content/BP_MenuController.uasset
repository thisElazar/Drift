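; BP_MenuController is an actor that sets up a procedural terrain preview, apparently for a menu.
; On BeginPlay it adds a GamePreviewManager component and copies its rotation, chunk size and noise settings into it.
; Graphs for applying, regenerating and resetting terrain are never triggered, and the Tick gate drives nothing.
; FUpdateTerrainParameters pushes chunk size and height variation and prints a debug string, but assigns NoiseScale to itself.
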(event EventBeginPlay
  (bind _returnvalue (Game|AddComponentbyClass "/Script/TerrAI.GamePreviewManager"))
  (Variables|/Script/TerrAI.GamePreviewManager|SetbEnableRotation _returnvalue (Variables|Default|GetEnableRotation))
  (Variables|/Script/TerrAI.GamePreviewManager|SetRotationSpeed _returnvalue (Variables|Default|GetRotationSpeed))
  (Variables|/Script/TerrAI.GamePreviewManager|SetPreviewChunkSize _returnvalue (Variables|Default|GetChunkSize))
  (Variables|/Script/TerrAI.GamePreviewManager|SetHeightVariation _returnvalue (Variables|Default|GetHeightVariation))
  (Variables|/Script/TerrAI.GamePreviewManager|SetNoiseScale _returnvalue (Variables|Default|GetNoiseScale))
  (Utilities|FlowControl|Gate true) ; enters at Open
)

(event Collision|EventActorBeginOverlap
  (params (OtherActor :type Actor%20Object%20Reference)))

(event EventTick
  (params (DeltaSeconds :type Float%20%28single-precision%29))
  (Utilities|FlowControl|Gate true))

(fn ConstructionScript)

(fn FUpdateTerrainParameters
  (bind _returnvalue (Actor|GetComponentbyClass "/Script/TerrAI.GamePreviewManager"))
  (Variables|/Script/TerrAI.GamePreviewManager|SetPreviewChunkSize _returnvalue (Variables|Default|GetChunkSize))
  (Variables|/Script/TerrAI.GamePreviewManager|SetHeightVariation _returnvalue (Variables|Default|GetHeightVariation))
  (Variables|Default|SetNoiseScale (Variables|Default|GetNoiseScale))
  (Development|PrintString "fUpdate Terrain Parameters Activated" true true "(R=1.000000,G=0.567316,B=0.107671,A=1.000000)"))