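; BP_TerrainController is a terrain controller Blueprint meant to locate a DynamicTerrain actor in the level.
; BeginPlay calls its parent, prints a debug message and gathers all DynamicTerrain actors.
; The follow-up logic, which sets TargetTerrain to the first result or spawns a terrain if none exists, is disconnected and never runs.
; Tick, overlap and construction script are empty.
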(event Collision|EventActorBeginOverlap
  (params (OtherActor :type Actor%20Object%20Reference)))

(event EventTick
  (params (DeltaSeconds :type Float%20%28single-precision%29)))

(event EventBeginPlay
  (|CallParentFunction)
  (Development|PrintString "Blueprint TerrainController BeginPlay!")
  (bind _outactors (Actor|GetAllActorsOfClass "/Script/TerrAI.DynamicTerrain")))

(fn ConstructionScript)